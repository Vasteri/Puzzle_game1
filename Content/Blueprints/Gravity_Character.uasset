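; Player character pawn with switchable global custom gravity, plus movement, camera, jump and sprint input.
; BeginPlay configures the player pawn's movement component for downward custom gravity, standing aligned to surface normals and falling along gravity.
; R toggles variant gravity, swapping those orientation modes and restoring downward gravity when turned off.
; While variant gravity is on, Q, E and F point global gravity up, down or along +Y.
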(event `self.ReceiveBeginPlay`
  (bind _ascustom_pawn (cast `CustomPawn` (`GameplayStatics.GetPlayerPawn` 0)))
  (bind _movementcomponent (`CustomPawn.MovementComponent` _ascustom_pawn))
  (set `CustomMovementComponent.GravitySwitchDelay` 1.0 _movementcomponent)
  (set `CustomMovementComponent.GravityScale` 3.0 _movementcomponent)
  (set `CustomMovementComponent.StandingVerticalOrientation` "EVO_SurfaceNormal" _movementcomponent)
  (set `CustomMovementComponent.FallingVerticalOrientation` "EVO_GravityDirection" _movementcomponent)
  (set `CustomMovementComponent.CustomGravityType` "EGT_GlobalCustom" _movementcomponent)
  (set `self.Variant_Gravity` false)
  (`CustomGravityManager.SetGlobalCustomGravityDirection` (`KismetMathLibrary.MakeVector` 0.0 0.0 -1.0)))

(event `InputAxis|Right_left`
  (params (AxisValue :type "Float (single-precision)"))
  (`self.AddRightMovementInput` AxisValue))

(event `Key|R`
  (params (Key :type "Key Structure"))
  (:`Pressed`
    (if (`self.Variant_Gravity`)
      (set `self.Variant_Gravity` false)
      (bind _movementcomponent (`CustomPawn.MovementComponent` (stale `self.ReceiveBeginPlay` _ascustom_pawn)))
      (set `CustomMovementComponent.StandingVerticalOrientation` "EVO_SurfaceNormal" _movementcomponent)
      (set `CustomMovementComponent.FallingVerticalOrientation` "EVO_GravityDirection" _movementcomponent)
      (`CustomGravityManager.SetGlobalCustomGravityDirection` (`KismetMathLibrary.MakeVector` 0.0 0.0 -1.0))
      (else
        (set `self.Variant_Gravity` true)
        (set `CustomMovementComponent.StandingVerticalOrientation` "EVO_GravityDirection" _movementcomponent)
        (set `CustomMovementComponent.FallingVerticalOrientation` "EVO_SurfaceNormal" _movementcomponent)))))

(event `InputAxis|Up_down`
  (params (AxisValue :type "Float (single-precision)"))
  (`self.AddForwardMovementInput` AxisValue))

(event `Key|Q`
  (params (Key :type "Key Structure"))
  (:`Pressed`
    (if (`self.Variant_Gravity`)
      (`CustomGravityManager.SetGlobalCustomGravityDirection` (`KismetMathLibrary.MakeVector` 0.0 0.0 1.0)))))

(event `InputAxis|Rotation_X`
  (params (AxisValue :type "Float (single-precision)"))
  (`self.AddCameraYawInput` 1.0 AxisValue))

(event `Key|LeftShift`
  (params (Key :type "Key Structure"))
  (:`Pressed`
    (`self.Sprint`))
  (:`Released`
    (`self.StopSprint`)))

(event `InputAction|Jump`
  (params (Key :type "Key Structure"))
  (:`Pressed`
    (`self.Jump`)))

(event `InputAxis|Rotation_Y`
  (params (AxisValue :type "Float (single-precision)"))
  (`self.AddCameraPitchInput` 1.0 AxisValue))

(event `Key|E`
  (params (Key :type "Key Structure"))
  (:`Pressed`
    (if (`self.Variant_Gravity`)
      (`CustomGravityManager.SetGlobalCustomGravityDirection` (`KismetMathLibrary.MakeVector` 0.0 0.0 -1.0)))))

(event `Key|F`
  (params (Key :type "Key Structure"))
  (:`Pressed`
    (if (`self.Variant_Gravity`)
      (`CustomGravityManager.SetGlobalCustomGravityDirection` (`KismetMathLibrary.MakeVector` 0.0 1.0 0.0)))))

(fn `UserConstructionScript`)